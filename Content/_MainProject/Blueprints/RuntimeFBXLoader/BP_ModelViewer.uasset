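; Actor that displays a runtime-loaded model, likely FBX, from supplied ModelData.
; InitializeModel applies an axis-corrected, upscaled root transform, then builds a procedural mesh component per mesh entry, each with a dynamic material fed color, metallic and textures.
; CleanMeshComponents only empties the tracking array, without destroying components.
; Tick triggers a throttled update on movement, but its loop is empty; render/collision refresh and Nanite static-mesh conversion are disconnected.
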(event Custom|Generate%20Mesh%20Components
  (bind _modeldata (Variables|Default|GetModelData))
  (if (.bsuccess _modeldata)
    (for _array_element (.meshmatinfo _modeldata)
      (Variables|Default|SetArray%20Element%20F%20Material%20Data (.fmaterialdata _array_element))
      (bind _returnvalue (AddComponent|AddProceduralMeshComponent false (.relativetransform _array_element)))
      (bind _output_get (Variables|Default|SetNewProcMeshComp _returnvalue))
      (Utilities|FlowControl|Sequence
        (:then_0
          (Variables|/Script/Engine.ActorComponent|SetComponentTags _output_get (Utilities|Array|MakeArray (Utilities|String|StringToName (Utilities|String|Append (.tmeshname _array_element) "_ProcMesh"))))
          (Transformation|SetMobility _output_get "Movable")
          (Rendering|SetCastShadow _output_get true)
          (Rendering|SetAffectDistanceFieldLighting _output_get true)
          (Class|PrimitiveComponent|SetAffectDynamicIndirectLighting _output_get true)
          (Collision|SetCollisionResponsetoAllChannels _output_get "ECR_Ignore"))
        (:then_1
          (Class|ProceduralMeshComponent|CreateMeshSectionLinearColor _output_get 0 (.vertices _array_element) (.triangles _array_element) (.normals _array_element) (.uv0 _array_element) 0 0 0 (.vertexcolors _array_element) (.tangents _array_element) true false)
          (bind _returnvalue_2 (Rendering|Material|CreateDynamicMaterialInstance (Variables|Default|GetParentMaterial) "None" "None" :!class /Script/Engine.KismetMaterialLibrary))
          (bind _output_get_2 (Variables|Default|SetDynamicMat _returnvalue_2))
          (Rendering|Material|SetMaterial (Variables|Default|GetNewProcMeshComp) 0 _output_get_2)
          (CallFunction|ConfigMaterial)
          (Utilities|Array|Add (Variables|Default|GetMeshComponents) (Variables|Default|GetNewProcMeshComp)))))))

(event Custom|Initialize%20Model
  (params (ModelData :type Modeld%20Material%20Data%20Structure) (ModelRootTransform :type Transform))
  (Variables|Default|SetModelData ModelData)
  (bind _output_get (Variables|Default|SetRootTransform (Math|Transform|MakeTransform (.location ModelRootTransform) (Math|Rotator|MakeRotator (+ (.roll (.rotation ModelRootTransform)) -9e+01) (.pitch (.rotation ModelRootTransform)) (+ (.yaw (.rotation ModelRootTransform)) 1.8e+02)) (* (.scale ModelRootTransform) (Math|Conversions|ToVector(Float) 1e+01)))))
  (CallFunction|CleanMeshComponents)
  (Transformation|SetActorTransform _output_get)
  (CallFunction|GenerateMeshComponents))

(event Custom|Update%20Model%20Transform
  (if (> (- (Utilities|Time|GetGameTimeinSeconds) (Variables|Default|GetLastUpdateTime)) 0.03) ; Only update every 3 FPS
    (for _array_element (Variables|Default|GetMeshComponents)
      _)))

(event EventBeginPlay
  (Variables|Default|SetLastLocation (Transformation|GetActorLocation))
  (Variables|Default|SetLastUpdateTime (Utilities|Time|GetGameTimeinSeconds))
  (Variables|Default|SetIsFirstRun false))

(event EventTick
  (params (DeltaSeconds :type Float%20%28single-precision%29))
  (bind _returnvalue (Transformation|GetActorLocation))
  (if (not (Variables|Default|GetIsFirstRun))
    (if (> (Math|Vector|Distance(Vector) _returnvalue (Variables|Default|GetLastLocation)) 1.0)
      (CallFunction|UpdateModelTransform)
      (Variables|Default|SetLastLocation _returnvalue))))

(fn ConstructionScript)

(fn CleanMeshComponents
  (bind _meshcomponents (Variables|Default|GetMeshComponents))
  (for _array_element _meshcomponents
    (Utilities|Array|RemoveItem _meshcomponents _array_element))
  (Utilities|Array|Clear (Variables|Default|GetMeshComponents)))

(fn ConfigMaterial
  (bind _array_element_f_material_data (Variables|Default|GetArray%20Element%20F%20Material%20Data))
  (bind _dynamicmat (Variables|Default|GetDynamicMat))
  (Rendering|Material|SetVectorParameterValue _dynamicmat "BaseColor" (.basecolor _array_element_f_material_data) :!class /Script/Engine.MaterialInstanceDynamic)
  (Rendering|Material|SetScalarParameterValue _dynamicmat "Metallic" (.metallic _array_element_f_material_data) :!class /Script/Engine.MaterialInstanceDynamic)
  (Utilities|IsValid (.basecolortextures _array_element_f_material_data)
    (:Is%20Valid
      (Rendering|Material|SetTextureParameterValue _dynamicmat "BaseColorTexture" (.basecolortextures _array_element_f_material_data))
      (Utilities|IsValid (.normaltextures _array_element_f_material_data)
        (:Is%20Valid
          (Rendering|Material|SetTextureParameterValue _dynamicmat "NormalTexture" (.normaltextures _array_element_f_material_data))
          (return))
        (:Is%20Not%20Valid
          (return))))
    (:Is%20Not%20Valid
      (return))))